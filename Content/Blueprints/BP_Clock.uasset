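; BP_Clock is a clock that displays the current system time as HH:MM:SS on its CurrentTime text.
; Every Tick it reads Now(), zero-pads hour, minute and second, then joins them with colons.
; Hours use modulo 12 with no AM/PM marker, so noon and midnight display as 00.
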(event EventTick
  (params (DeltaSeconds :type Float%20%28single-precision%29))
  (bind _returnvalue (Math|DateTime|Now))
  (bind _returnvalue_2 (Class|KismetMathLibrary|GetHour _returnvalue))
  (bind _returnvalue_3 (Class|KismetMathLibrary|GetMinute _returnvalue))
  (bind _returnvalue_4 (Class|KismetMathLibrary|GetSecond _returnvalue))
  (bind _returnvalue_5 (Math|Integer|%(Integer) _returnvalue_2 12))
  ;[1 1 1] Add Leading Zeros
  (if (< _returnvalue_5 10)
    (Variables|Default|SetHour (Utilities|Text|FormatText "0{A}" _returnvalue_5))
    (else
      (Variables|Default|SetHour (Utilities|Text|ToText(Integer) _returnvalue_5))))
  (if (< _returnvalue_3 10)
    (Variables|Default|SetMinutes (Utilities|Text|FormatText "0{A}" _returnvalue_3))
    (else
      (Variables|Default|SetMinutes (Utilities|Text|ToText(Integer) _returnvalue_3))))
  (if (< _returnvalue_4 10)
    (Variables|Default|SetSeconds (Utilities|Text|FormatText "0{A}" _returnvalue_4))
    (else
      (Variables|Default|SetSeconds (Utilities|Text|ToText(Integer) _returnvalue_4))))
  (Rendering|Components|TextRender|SetText (Variables|Default|GetCurrent%20Time) (Utilities|Text|FormatText "{A}:{B}:{C}" (Variables|Default|GetHour) (Variables|Default|GetMinutes) (Variables|Default|GetSeconds))))

(fn ConstructionScript)