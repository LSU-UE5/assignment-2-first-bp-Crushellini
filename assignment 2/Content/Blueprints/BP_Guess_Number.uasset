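; Number-guessing toy Blueprint: Space bar presses count a guess up from zero toward a visible random target between 0 and 20.
; BeginPlay rolls the target and writes both numbers to text components; each press increments the guess and reruns the shared display-and-compare chain.
; A match swaps both numbers for the YouWin text, then after a short delay loops back to start a new round.
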(event EventBeginPlay
  (bind _output_get (Variables|Default|SetGuessInt 0 :!label _label))
  (Rendering|Components|TextRender|SetText (Variables|Default|GetGuess) (Utilities|Text|ToText(Integer) _output_get))
  ;[1 1 1] Set Random Int
  (bind _output_get_2 (Variables|Default|SetRandomInt (Math|Random|RandomIntegerinRange 0 20)))
  (Rendering|Components|TextRender|SetText (Variables|Default|GetRandInt) (Utilities|Text|ToText(Integer) _output_get_2))
  ;[1 1 1] Increment Guess
  (Rendering|Components|TextRender|SetText (Variables|Default|GetGuess) (Utilities|Text|ToText(Integer) (stale Input|KeyboardEvents|SpaceBar _result)))
  ;[1 1 1] Reset Visibilities
  (Rendering|SetVisibility (Variables|Default|GetYouWin) false false)
  (Rendering|SetVisibility (Variables|Default|GetGuess) true false)
  (Rendering|SetVisibility (Variables|Default|GetRandInt) true false)
  (if (== (Variables|Default|GetRandomInt) (Variables|Default|GetGuessInt))
    ;[1 1 1] Win Text
    (Rendering|SetVisibility (Variables|Default|GetYouWin) true false)
    (Rendering|SetVisibility (Variables|Default|GetGuess) false false)
    (Rendering|SetVisibility (Variables|Default|GetRandInt) false false)
    (Utilities|FlowControl|Delay 0.5)
    (goto _label)))

(event Input|KeyboardEvents|SpaceBar
  (params (Key :type Key%20Structure :default "None"))
  ;[1 1 1] Increment Guess
  (:Pressed
    (bind _result (Math|Integer|IncrementInt (Variables|Default|GetGuessInt))
      (:%20%20
        (Rendering|Components|TextRender|SetText (Variables|Default|GetGuess) (Utilities|Text|ToText(Integer) _result) :!label _label)
        ;[1 1 1] Reset Visibilities
        (Rendering|SetVisibility (Variables|Default|GetYouWin) false false)
        (Rendering|SetVisibility (Variables|Default|GetGuess) true false)
        (Rendering|SetVisibility (Variables|Default|GetRandInt) true false)
        (if (== (Variables|Default|GetRandomInt) (Variables|Default|GetGuessInt))
          ;[1 1 1] Win Text
          (Rendering|SetVisibility (Variables|Default|GetYouWin) true false)
          (Rendering|SetVisibility (Variables|Default|GetGuess) false false)
          (Rendering|SetVisibility (Variables|Default|GetRandInt) false false)
          (Utilities|FlowControl|Delay 0.5)
          (bind _output_get (Variables|Default|SetGuessInt 0))
          (Rendering|Components|TextRender|SetText (Variables|Default|GetGuess) (Utilities|Text|ToText(Integer) _output_get))
          ;[1 1 1] Set Random Int
          (bind _output_get_2 (Variables|Default|SetRandomInt (Math|Random|RandomIntegerinRange 0 20)))
          (Rendering|Components|TextRender|SetText (Variables|Default|GetRandInt) (Utilities|Text|ToText(Integer) _output_get_2))
          (goto _label))))))

(fn ConstructionScript)